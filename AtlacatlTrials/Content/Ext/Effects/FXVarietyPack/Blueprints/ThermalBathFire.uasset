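; ThermalBathFire is a fire effect actor from FXVarietyPack, apparently derived from a projectile template.
; BeginPlay spawns a colored shot shockwave emitter and runs a timeline that updates SpeedCorrect.
; The movement, hit effect and timed destruction logic is disconnected and never runs, leaving Tick and overlap events empty.
; ActivateParticles provides a function to switch on the FX1 particle component.
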(event EventBeginPlay
  (bind _defaultsceneroot (Variables|Default|GetDefaultSceneRoot))
  ;[1 1 1] spawn shot shockwave
  (bind _returnvalue (Effects|SpawnEmitteratLocation "/Game/Ext/Effects/FXVarietyPack/Particles/P_ky_shotShockwave.P_ky_shotShockwave" (Transformation|GetWorldLocation _defaultsceneroot) (Transformation|GetWorldRotation _defaultsceneroot) "1.000000,1.000000,1.000000" false))
  (Effects|Components|ParticleSystem|SetVectorParameter _returnvalue "color" (Math|Conversions|ToVector(LinearColor) (Variables|Default|Getcolor)))
  ;[1 1 1] effect move correct
  (bind _valuecorrect (Timeline|Timeline_0 Play)
    (:Update
      (Variables|Default|SetspeedCorrect _valuecorrect))))

(event Collision|EventActorBeginOverlap
  (params (OtherActor :type Actor%20Object%20Reference))
  ;[1 1 1] spawn collison fx
)

(event EventTick
  (params (DeltaSeconds :type Float%20%28single-precision%29))
  ;[1 1 1] duration increment for control
)

(fn ConstructionScript)

(fn ActivateParticles
  (Components|Activation|Activate (Variables|Default|GetFX1) false))