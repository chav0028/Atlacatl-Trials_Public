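; BP_ThermalBath is an interactable thermal bath actor that heats up when the player interacts with it.
; Interact disables further interaction by ignoring a trace channel on its Box, plays a fire sound and activates steam particles.
; If the referenced fire particles actor is valid, it activates that too and runs a timeline that fades in the point light and, when set, a post-process volume's blend weight.
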(event EventInteract
  (params (aUser :type Actor%20Object%20Reference))
  ;[1 1 1] Disable any more interaction
  (Collision|SetCollisionResponsetoChannel (Variables|Default|GetBox) "ECC_GameTraceChannel2" "ECR_Ignore")
  ;[1 1 1] Play sound
  (Audio|PlaySoundatLocation "/Game/Ext/Audio/Game/Cue_Fire.Cue_Fire" (Transformation|GetWorldLocation (Variables|Default|GetPointLight)) "0, 0, 0" 0.5 1.0 0.0 "/Game/AudioSettings/DefaultAttenuation.DefaultAttenuation" 0 0)
  ;[1 1 1] Show components
  (Components|Activation|Activate (Variables|Default|GetSteamParticles) false)
  ;[1 1 1] Show fire particles
  (bind _m_fireparticles (Variables|Default|Getm_fireParticles)
    (:then
      (Default|ActivateParticles _m_fireparticles)
      ;[1 1 1] Activate effects slowly through timeline
      (bind _0to1 (Timeline|LerpPostProcessVolume PlayFromStart)
        (:Update
          (Rendering|Components|Light|SetIntensity (Variables|Default|GetPointLight) (Math|Float|Lerp 0.0 (Variables|Default|Getm_targetLightIntensity) _0to1))
          (bind _m_postprocessvolume (Variables|Default|Getm_postProcessVolume)
            (:then
              (Variables|/Script/Engine.PostProcessVolume|SetBlendWeight _m_postprocessvolume _0to1))
            (:else)))))
    (:else)))

(fn ConstructionScript)