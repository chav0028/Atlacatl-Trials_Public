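; BP_FracturedSkull is a destructible skull target that shatters when broken by an impact and reports the hit to the game mode.
; Break runs once on a blocking hit, moving a radial force to the impact point and scaling it by the breaker's speed.
; It then enables physics on the destructible component, fires the impulse, notifies FirstPersonGameMode that a target was shot, and plays a breaking obsidian sound.
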(event EventBeginPlay)

(event EventBreak
  (params (aBreaker :type Actor%20Object%20Reference) (aHit :type Hit%20Result%20Structure))
  (bind (_bblockinghit _binitialoverlap _time _distance _location) (Collision|BreakHitResult aHit))
  (bind _returnvalue (Transformation|GetVelocity aBreaker))
  (bind _m_forcespeedmultiplier (Variables|Default|Getm_forceSpeedMultiplier))
  (bind _radialforce (Variables|Default|GetRadialForce))
  (bind _returnvalue_2 (Math|Vector|VectorLength _returnvalue))
  (bind _returnvalue_3 (* _returnvalue_2 _m_forcespeedmultiplier))
  ;[1 1 1] Check collision is valid
  (if (not (Variables|Default|Getm_isBroken))
    (if _bblockinghit
      ;[1 1 1] Prepare radial force according to impact
      (Transformation|SetWorldLocation (Variables|Default|GetRadialForce) _location false true)
      (Variables|/Script/Engine.RadialForceComponent|SetImpulseStrength _radialforce _returnvalue_3)
      (Variables|/Script/Engine.RadialForceComponent|SetForceStrength _radialforce _returnvalue_3)
      ;[1 1 1] Break object
      (Physics|SetSimulatePhysics (Variables|Default|GetDestructibleComponent) true)
      (Class|RadialForceComponent|FireImpulse (Variables|Default|GetRadialForce))
      (Variables|Default|Setm_isBroken true)
      ;[1 1 1] Notify target was shot
      (bind _asfirst_person_game_mode (Utilities|Casting|CastToFirstPersonGameMode (Game|GetGameMode)))
      (Default|MightTargetShot _asfirst_person_game_mode)
      ;[1 1 1] Play sound
      (Audio|PlaySoundatLocation "/Game/Ext/Audio/Game/Cue_BreakingObsidian.Cue_BreakingObsidian" _location "0, 0, 0" 1.0 1.0 0.0 "/Game/AudioSettings/DefaultAttenuation.DefaultAttenuation" 0 0))))

(fn ConstructionScript)