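; BP_OfferingBowl is an interactable offering bowl for a ritual step that stays locked until the game mode reports all exploration goals finished.
; Once unlocked, interacting reveals the knife, cocoa and corn meshes, reports the ritual step to FirstPersonGameMode, disables further interaction through the collision channel and plays a sound.
; While locked, interacting re-shows a timed warning widget created at BeginPlay.
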(event Custom|ExplorationGoalsFinished
  ;[1 1 1] Create widget and suscribe to game mode events
  (Variables|Default|Setm_canBeUsed true))

(event EventBeginPlay
  ;[1 1 1] Create widget and suscribe to game mode events
  (bind _returnvalue (UserInterface|CreateWidget "/Game/Blueprints/UI/Prompts/BlockingMessage.BlockingMessage_C" (Game|GetPlayerController 0) "You need to collect the required items before making an offer" 1.0))
  (Variables|Default|Setm_warningMessageWidget _returnvalue)
  (bind _asfirst_person_game_mode (Utilities|Casting|CastToFirstPersonGameMode (Game|GetGameMode)))
  (EventDispatchers|BindEventtoAllExplorationGoalsFinished _asfirst_person_game_mode (delegate Custom|ExplorationGoalsFinished)))

(event EventInteract
  (params (aUser :type Actor%20Object%20Reference))
  (bind _m_warningmessagewidget (Variables|Default|Getm_warningMessageWidget))
  ;[1 1 1] If usable, show items, if not, show warning message
  (if (Variables|Default|Getm_canBeUsed)
    (Rendering|SetVisibility (Variables|Default|GetJadeKnife) true false)
    (Rendering|SetVisibility (Variables|Default|GetCocoa) true false)
    (Rendering|SetVisibility (Variables|Default|GetCorn) true false)
    (bind _asfirst_person_game_mode (Utilities|Casting|CastToFirstPersonGameMode (Game|GetGameMode)))
    (Default|FinishedExplorationRitualStep _asfirst_person_game_mode "NewEnumerator1")
    (Collision|SetCollisionResponsetoChannel (Variables|Default|GetInteractionBox) "ECC_GameTraceChannel2" "ECR_Ignore")
    (Audio|PlaySoundatLocation "/Game/Ext/Audio/UI/Cue_ItemCollected.Cue_ItemCollected" (Transformation|GetWorldLocation (Variables|Debug|GetStaticMeshComponent)) "0, 0, 0" 1.0 1.0 0.0 "/Game/AudioSettings/DefaultAttenuation.DefaultAttenuation" 0 0)
    (else
      (Widget|RemovefromParent _m_warningmessagewidget)
      (UserInterface|Viewport|AddtoViewport _m_warningmessagewidget 0))))

(fn ConstructionScript)