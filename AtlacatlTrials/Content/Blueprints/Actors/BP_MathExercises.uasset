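; BP_MathExercises is an interactable actor that opens a number puzzle UI for the player.
; It creates the PuzzleNumbers widget on BeginPlay with a self reference, then on Interact shows it with UI-only input and plays a sound.
; SetInteractivity toggles the detection component's trace-channel response and opens or closes the game mode's menu state.
; DisableInteractivity blocks further interaction without touching the menu.
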(event EventBeginPlay
  ;[1 1 1] Create UI
  (bind _returnvalue (UserInterface|CreateWidget "/Game/Blueprints/UI/PuzzleNumbers.PuzzleNumbers_C" (Game|GetPlayerController 0) self))
  (Variables|Default|Setm_puzzleUI _returnvalue))

(event EventInteract
  (params (aUser :type Actor%20Object%20Reference))
  (bind _m_puzzleui (Variables|Default|Getm_puzzleUI))
  ;[1 1 1] Show UI
  (Input|SetInputModeUIOnly (Game|GetPlayerController 0) _m_puzzleui "DoNotLock")
  (UserInterface|Viewport|AddtoViewport _m_puzzleui 0)
  (CallFunction|SetInteractivity false)
  (Audio|PlaySoundatLocation "/Game/Ext/Audio/Game/Cue_Correct.Cue_Correct" (Transformation|GetWorldLocation (Variables|Debug|GetStaticMeshComponent)) "0, 0, 0" 1.0 1.0 0.0 0 0 0))

(fn ConstructionScript)

(fn SetInteractivity
  (params (aIsInteractable :type Boolean))
  (bind _interactabledetection (Variables|Default|GetInteractableDetection))
  ;[1 1 1] Set collision response to make object interactable or not
  (if aIsInteractable
    (Collision|SetCollisionResponsetoChannel _interactabledetection "ECC_GameTraceChannel2" "ECR_Block")
    (bind _asfirst_person_game_mode (Utilities|Casting|CastToFirstPersonGameMode (Game|GetGameMode)))
    (Default|CloseMenu _asfirst_person_game_mode)
    (else
      (Collision|SetCollisionResponsetoChannel _interactabledetection "ECC_GameTraceChannel2" "ECR_Ignore")
      (bind _asfirst_person_game_mode_2 (Utilities|Casting|CastToFirstPersonGameMode (Game|GetGameMode)))
      (Default|OpenMenu _asfirst_person_game_mode_2))))

(fn DisableInteractivity
  (Collision|SetCollisionResponsetoChannel (Variables|Default|GetInteractableDetection) "ECC_GameTraceChannel2" "ECR_Ignore"))