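; BP_InformationTrigger is a trigger actor that lets the player view a piece of information while standing inside it.
; At BeginPlay it creates an InfoPrompt widget titled from its CInformation component.
; Player overlap enables input and shows the prompt; leaving disables input and hides both prompt and info.
; The Information action, ignored while the game mode reports a menu open, toggles the component's info display, swapping it with the prompt.
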(event Collision|EventActorBeginOverlap
  (params (OtherActor :type Actor%20Object%20Reference))
  ;[1 1 1] Add prompt to screen
  (Utilities|Casting|CastToFirstPersonCharacter OtherActor)
  (Input|EnableInput (Game|GetPlayerController 0))
  (UserInterface|Viewport|AddtoViewport (Variables|Default|Getm_promptWidget) 0))

(event EventBeginPlay
  ;[1 1 1] Create widget
  (bind _returnvalue (UserInterface|CreateWidget "/Game/Blueprints/UI/Prompts/InfoPrompt.InfoPrompt_C" (Game|GetPlayerController 0) (Default|GetInformationTitle (Variables|Default|GetCInformation))))
  (Variables|Default|Setm_promptWidget _returnvalue))

(event Collision|EventActorEndOverlap
  (params (OtherActor :type Actor%20Object%20Reference))
  ;[1 1 1] Remove prompt from screen
  (Utilities|Casting|CastToFirstPersonCharacter OtherActor)
  (Input|DisableInput (Game|GetPlayerController 0))
  (Widget|RemovefromParent (Variables|Default|Getm_promptWidget))
  (Default|HideInfo (Variables|Default|GetCInformation)))

(event Input|ActionEvents|InputActionInformation
  (params (Key :type Key%20Structure))
  (bind _cinformation (Variables|Default|GetCInformation))
  (bind _m_promptwidget (Variables|Default|Getm_promptWidget))
  ;[1 1 1] Check player is not in other menu
  (:Pressed
    (bind _asfirst_person_game_mode (Utilities|Casting|CastToFirstPersonGameMode (Game|GetGameMode)))
    (bind _aisinmenu (Default|GetIsinMenu _asfirst_person_game_mode))
    (if (not _aisinmenu)
      ;[1 1 1] Show/hide information
      (if (Default|GetIsInformationShowing _cinformation)
        (Default|HideInfo _cinformation)
        (UserInterface|Viewport|AddtoViewport _m_promptwidget 0)
        (else
          (Default|ShowInfo _cinformation)
          (Widget|RemovefromParent _m_promptwidget))))))

(fn ConstructionScript)