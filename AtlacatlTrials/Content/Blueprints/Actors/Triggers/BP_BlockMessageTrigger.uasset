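; Trigger actor that shows a BlockingMessage warning widget on screen when its collision component is overlapped.
; BeginPlay creates the widget once for player 0, passing in the configured text, display time and auto-close flag, and can start the actor disabled for testing.
; Begin overlap, with no check on the overlapping actor, adds the widget to the viewport.
; End overlap removes it only when auto-close is off.
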(event OnComponentBeginOverlap(CollisionComponent)
  (params (OverlappedComponent :type Primitive%20Component%20Object%20Reference) (OtherActor :type Actor%20Object%20Reference) (OtherComp :type Primitive%20Component%20Object%20Reference) (OtherBodyIndex :type Integer) (bFromSweep :type Boolean) (SweepResult :type Hit%20Result%20Structure%20%28by%20ref%29))
  ;[1 1 1] Show prompt
  (bind _m_messagewidget (Variables|Default|Getm_messageWidget)
    (:then
      (UserInterface|Viewport|AddtoViewport _m_messagewidget 0))
    (:else)))

(event OnComponentEndOverlap(CollisionComponent)
  (params (OverlappedComponent :type Primitive%20Component%20Object%20Reference) (OtherActor :type Actor%20Object%20Reference) (OtherComp :type Primitive%20Component%20Object%20Reference) (OtherBodyIndex :type Integer))
  ;[1 1 1] Hide prompt
  (if (not (Variables|Default|Getm_willAutoCloseMessage))
    (bind _m_messagewidget (Variables|Default|Getm_messageWidget)
      (:then
        (Widget|RemovefromParent _m_messagewidget))
      (:else))))

(event EventBeginPlay
  ;[1 1 1] Creae widget
  (bind _returnvalue (UserInterface|CreateWidget "/Game/Blueprints/UI/Prompts/BlockingMessage.BlockingMessage_C" (Game|GetPlayerController 0) (Variables|Default|Getm_messageShown) (Variables|Default|Getm_timeMessageShown) (Variables|Default|Getm_willAutoCloseMessage)))
  (Variables|Default|Setm_messageWidget _returnvalue)
  ;;[1 1 1] For testing, have the option to turn off this actor at start
  (if (Variables|Default|Getm_startDisabled)
    (CallFunction|SetActorEnabled self false)))

(fn ConstructionScript)