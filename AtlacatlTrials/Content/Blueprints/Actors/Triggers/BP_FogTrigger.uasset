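; Trigger volume actor that hides a referenced fog actor while the player is inside by changing the fog's start distance.
; Overlap begin and end play and reverse the FogStart timeline, which lerps between on and off distances, with no actor class filter.
; Shortly after BeginPlay, it snaps to the off distance if a FirstPersonCharacter already overlaps the collision component.
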(event EventBeginPlay
  ;[1 1 1] If player starts inside one of  this, hide fog
  ;;[1 1 1] Small delay to be sure actor was created
  (Utilities|FlowControl|Delay 0.1)
  (if (> (Utilities|Array|Length (Collision|GetOverlappingActors (Variables|Default|GetCollisionComponent) "/Game/Ext/FirstPerson/FirstPersonBP/Blueprints/FirstPersonCharacter.FirstPersonCharacter_C" :!class /Script/Engine.PrimitiveComponent)) 0)
    (bind _m_fog (Variables|Default|Getm_fog)
      (:then
        (Class|ExponentialHeightFogComponent|SetStartDistance (Variables|/Script/Engine.ExponentialHeightFog|GetComponent _m_fog) (Variables|Default|Getm_fogOffStartDistance)))
      (:else))))

(event Collision|EventActorBeginOverlap
  (params (OtherActor :type Actor%20Object%20Reference))
  ;[1 1 1] Hide or show fog
  (bind _lerp0to1 (Timeline|FogStart PlayFromStart)
    (:Update
      (bind _m_fog (Variables|Default|Getm_fog)
        (:then
          (Class|ExponentialHeightFogComponent|SetStartDistance (Variables|/Script/Engine.ExponentialHeightFog|GetComponent _m_fog) (Math|Float|Lerp (Variables|Default|Getm_fogOnStartDistance) (Variables|Default|Getm_fogOffStartDistance) _lerp0to1)))
        (:else)))))

(event Collision|EventActorEndOverlap
  (params (OtherActor :type Actor%20Object%20Reference))
  ;[1 1 1] Hide or show fog
  (bind _lerp0to1 (Timeline|FogStart ReverseFromEnd)
    (:Update
      (bind _m_fog (Variables|Default|Getm_fog)
        (:then
          (Class|ExponentialHeightFogComponent|SetStartDistance (Variables|/Script/Engine.ExponentialHeightFog|GetComponent _m_fog) (Math|Float|Lerp (Variables|Default|Getm_fogOnStartDistance) (Variables|Default|Getm_fogOffStartDistance) _lerp0to1)))
        (:else)))))

(fn ConstructionScript)