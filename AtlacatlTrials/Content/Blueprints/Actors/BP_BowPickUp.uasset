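; Bow pickup actor that gives the player the bow once a specific exploration ritual step, apparently the offering, has finished.
; It listens to the game mode's step-finished event to toggle whether it can be picked up.
; A valid interaction hides the mesh, enables the character's bow, reports the next finished step, ignores further interaction traces and plays a sound.
; Otherwise it re-adds a pre-created warning widget.
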(event Custom|RitualStepFinished
  (params (aRitualStep :type EExplorationRitual%20Enum :default "NewEnumerator1"))
  ;[1 1 1] Create widget and suscribe to game mode events
  (Variables|Default|Setm_canBePickedUp (Utilities|Enum|Equal(Enum) aRitualStep "NewEnumerator1")))

(event EventBeginPlay
  ;[1 1 1] Create widget and suscribe to game mode events
  (bind _returnvalue (UserInterface|CreateWidget "/Game/Blueprints/UI/Prompts/BlockingMessage.BlockingMessage_C" (Game|GetPlayerController 0) "You need to make an offering before picking up the bow" 1.0))
  (Variables|Default|Setm_warningMessageWidget _returnvalue)
  (bind _asfirst_person_game_mode (Utilities|Casting|CastToFirstPersonGameMode (Game|GetGameMode)))
  (EventDispatchers|BindEventtoExplorationRitualStepFinished _asfirst_person_game_mode (delegate Custom|RitualStepFinished)))

(event EventInteract
  (params (aUser :type Actor%20Object%20Reference))
  (bind _m_warningmessagewidget (Variables|Default|Getm_warningMessageWidget))
  ;[1 1 1] If usable, pick up bow, if not, show warning message
  (if (Variables|Default|Getm_canBePickedUp)
    (Rendering|SetVisibility (Variables|SkeletalMeshActor|GetSkeletalMeshComponent) false true)
    ;;[1 1 1] Add bow to player
    (bind _asfirst_person_character (Utilities|Casting|CastToFirstPersonCharacter aUser)
      (:then
        (Default|SetBowEnabled _asfirst_person_character true))
      (:CastFailed
        _))
    (bind _asfirst_person_game_mode (Utilities|Casting|CastToFirstPersonGameMode (Game|GetGameMode)))
    (Default|FinishedExplorationRitualStep _asfirst_person_game_mode "NewEnumerator4")
    (Collision|SetCollisionResponsetoChannel (Variables|Default|GetInteractionBox) "ECC_GameTraceChannel2" "ECR_Ignore")
    (Audio|PlaySoundatLocation "/Game/Ext/Audio/UI/Cue_ItemCollected.Cue_ItemCollected" (Transformation|GetWorldLocation (Variables|SkeletalMeshActor|GetSkeletalMeshComponent)) "0, 0, 0" 1.0 1.0 0.0 "/Game/AudioSettings/DefaultAttenuation.DefaultAttenuation" 0 0)
    (else
      (Widget|RemovefromParent _m_warningmessagewidget)
      (UserInterface|Viewport|AddtoViewport _m_warningmessagewidget 0))))

(fn ConstructionScript)