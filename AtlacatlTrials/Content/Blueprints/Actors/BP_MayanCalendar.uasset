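; Interactive Mayan calendar puzzle whose stone wheel the player rotates into the correct position.
; Interact plays a sound and timeline rotation, blocking GameTraceChannel2 interaction until it finishes.
; A delayed check, restarted by each interaction, tests whether DetectionBox overlaps the Step1Sphere target.
; A match reveals the completion decal, notifies FirstPersonGameMode, plays a success sound and disables further interaction.
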(event Custom|CheckRotationComplete
  ;[1 1 1] Evaluate if rotation completes a step
  (if (not (Variables|Default|Getm_isRotating))
    (CallFunction|EvaluateRotation)
    ;[1 1 1] Reenable object
    (Variables|Default|Setm_isRotating false)
    (if (not (Variables|Default|Getm_isStep1Done))
      (Collision|SetCollisionResponsetoChannel (Variables|Default|GetCollisionBox) "ECC_GameTraceChannel2" "ECR_Block"))))

(event EventInteract
  (params (aUser :type Actor%20Object%20Reference))
  ;[1 1 1] Disable object so that it can only rotate one space at a time (no multiclick)
  (Variables|Default|Setm_isRotating true)
  (Collision|SetCollisionResponsetoChannel (Variables|Default|GetCollisionBox) "ECC_GameTraceChannel2" "ECR_Ignore")
  (Utilities|Time|ClearandInvalidateTimerbyHandle (Variables|Default|Getm_checkTimer))
  ;[1 1 1] Play sound
  (Audio|PlaySoundatLocation "/Game/Ext/Audio/Game/Cue_rotatingStone.Cue_rotatingStone" (Transformation|GetWorldLocation (Variables|Default|GetArrowDecal)) "0, 0, 0" 1.0 1.0 0.0 "/Game/AudioSettings/DefaultAttenuation.DefaultAttenuation" 0 0)
  ;[1 1 1] Rotate object
  (bind _newtrack_0 (Timeline|RotationAnim PlayFromStart)
    (:Update
      (Transformation|AddLocalRotation (Variables|Default|GetCalendar%20Wheel) (Math|Rotator|MakeRotator 0.0 (* _newtrack_0 -1.0) 0.0) false false))
    (:Finished
      ;[1 1 1] Evaluate if rotation completes a step
      (bind _returnvalue (Utilities|Time|SetTimerbyEvent (delegate Custom|CheckRotationComplete) (Variables|Default|Getm_timeCheck)))
      (Variables|Default|Setm_checkTimer _returnvalue)
      ;[1 1 1] Reenable object
      (Variables|Default|Setm_isRotating false)
      (if (not (Variables|Default|Getm_isStep1Done))
        (Collision|SetCollisionResponsetoChannel (Variables|Default|GetCollisionBox) "ECC_GameTraceChannel2" "ECR_Block")))))

(fn ConstructionScript)

(fn EvaluateRotation
  ;[1 1 1] Get objects being selected
  (for _array_element (Class|PrimitiveComponent|GetOverlappingComponents (Variables|Default|GetDetectionBox))
    ;[1 1 1] Chek step 1
    (if (not (Variables|Default|Getm_isStep1Done))
      (if (== _array_element (Variables|Default|GetStep1Sphere))
        (Rendering|SetVisibility (Variables|Default|GetStep1DecalComplete) true false)
        (Variables|Default|Setm_isStep1Done true))))
  ;[1 1 1] If all steps were completed
  (if (Variables|Default|Getm_isStep1Done)
    (bind _asfirst_person_game_mode (Utilities|Casting|CastToFirstPersonGameMode (Game|GetGameMode)))
    (Default|FinishedMayanCalendarPuzzle _asfirst_person_game_mode)
    (Collision|SetCollisionResponsetoChannel (Variables|Default|GetCollisionBox) "ECC_GameTraceChannel2" "ECR_Ignore")
    (Audio|PlaySoundatLocation "/Game/Ext/Audio/Game/Cue_Correct.Cue_Correct" (Transformation|GetWorldLocation (Variables|Default|GetStep1DecalComplete)) "0, 0, 0" 1.0 1.0 0.0 "/Game/AudioSettings/DefaultAttenuation.DefaultAttenuation" 0 0)))