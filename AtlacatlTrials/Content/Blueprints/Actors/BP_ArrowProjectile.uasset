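; BP_ArrowProjectile is a physics-driven arrow that breaks targets or sticks into whatever it hits, with optional timed self-destruction.
; ReleaseArrow detaches it, enables physics and applies a forward impulse at the launch point.
; Once released, head hits break IBreakable actors or otherwise stop the arrow, attach it to the hit component and play a sound.
; Body hits also break targets for usability, but never stick the arrow.
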(event OnComponentHit(ArrowHead)
  (params (HitComponent :type Primitive%20Component%20Object%20Reference) (OtherActor :type Actor%20Object%20Reference) (OtherComp :type Primitive%20Component%20Object%20Reference) (NormalImpulse :type Vector :default "0, 0, 0") (Hit :type Hit%20Result%20Structure%20%28by%20ref%29))
  (if (Variables|Default|Getm_hasBeenReleased)
    (bind _asibreakable (Utilities|Casting|CastToIBreakable OtherActor)
      (:then
        ;[1 1 1] Make arrow break object
        (Default|Break _asibreakable self Hit))
      (:CastFailed
        ;[1 1 1] Stop arrow
        (Physics|SetPhysicsLinearVelocity (Variables|Debug|GetStaticMeshComponent) "0, 0, 0" false "None")
        (Physics|SetSimulatePhysics (Variables|Debug|GetStaticMeshComponent) false)
        (Transformation|AttachComponentToComponent OtherComp "None" "KeepWorld" "KeepWorld" "KeepWorld" true)
        (Collision|SetCollisionResponsetoAllChannels (Variables|Default|GetArrowHead) "ECR_Ignore")
        (Audio|PlaySoundatLocation "/Game/Ext/Audio/Game/Cue_ArrowHit.Cue_ArrowHit" (.ImpactPoint (Collision|BreakHitResult Hit)) "0, 0, 0" 1.0 1.0 0.0 "/Game/AudioSettings/DefaultAttenuation.DefaultAttenuation" 0 0)))))

(event OnComponentHit(ArrowBody)
  (params (HitComponent :type Primitive%20Component%20Object%20Reference) (OtherActor :type Actor%20Object%20Reference) (OtherComp :type Primitive%20Component%20Object%20Reference) (NormalImpulse :type Vector :default "0, 0, 0") (Hit :type Hit%20Result%20Structure%20%28by%20ref%29))
  ;[1 1 1] For usability, the arrow  body may also break targets, but won't stick the arrow
  (if (Variables|Default|Getm_hasBeenReleased)
    (bind _asibreakable (Utilities|Casting|CastToIBreakable OtherActor))
    (Default|Break _asibreakable 0 Hit)))

(event EventBeginPlay
  ;[1 1 1] Auto destroy after certain time
  (if (Variables|Default|Getm_autoDestroy)
    (Actor|SetLifeSpan (Variables|Default|Getm_autoDestroyTime))))

(fn ConstructionScript)

(fn ReleaseArrow
  (params (aLaunchForce :type Float%20%28single-precision%29))
  ;[1 1 1] Enable collisions and add force
  (Variables|Default|Setm_hasBeenReleased true)
  (Transformation|DetachFromActor "KeepWorld" "KeepWorld" "KeepWorld")
  (Physics|SetSimulatePhysics (Variables|Debug|GetStaticMeshComponent) true)
  (Physics|AddImpulseatLocation (Variables|Debug|GetStaticMeshComponent) (* (Math|Vector|GetForwardVector (Variables|Debug|GetStaticMeshComponent)) aLaunchForce) (Transformation|GetWorldLocation (Variables|Default|GetLaunchLocation)) "None"))