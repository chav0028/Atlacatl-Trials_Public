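; Actor component that lets its owner interact with objects in the world through the IInteractable interface.
; TraceInteractables runs a line trace from a given start and direction, limited by the interaction range, and returns the hit.
; UseInteractables takes that hit and calls Interact on the hit actor and on any of its components implementing the interface, passing the owner as the interactor.
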(fn TraceInteractables
  (params (aTraceStartPosition :type Vector) (aTraceDirection :type Vector))
  ;[1 1 1] Line trace for interactables objects
  (bind (_outhit _returnvalue) (Collision|LineTraceByChannel aTraceStartPosition (+ aTraceStartPosition (* aTraceDirection (Variables|Default|Getm_interactionRange))) "TraceTypeQuery3" false 0 "None"))
  (return _outhit _returnvalue))

(fn UseInteractables
  (params (aInteractablesDetected :type Hit%20Result%20Structure))
  (bind (_bblockinghit _binitialoverlap _time _distance _location _impactpoint _normal _impactnormal _physmat _hitactor) (Collision|BreakHitResult aInteractablesDetected))
  ;[1 1 1] If something was hit
  (if _bblockinghit
    ;[1 1 1] If actor implements interface
    (bind _asiinteractable (Utilities|Casting|CastToIInteractable _hitactor)
      (:then
        (Default|Interact _asiinteractable (Components|GetOwner)))
      (:CastFailed
        _))
    ;[1 1 1] If actor has an actor component that implements the interface
    (for _array_element (Class|Actor|GetComponentsbyInterface _hitactor "/Game/Blueprints/Interfaces/IInteractable.IInteractable_C")
      (bind _asiinteractable_2 (Utilities|Casting|CastToIInteractable _array_element))
      (Default|Interact _asiinteractable_2 (Components|GetOwner)))))