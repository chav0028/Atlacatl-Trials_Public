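; Actor component that gives its owning actor an information panel that can be shown or hidden on screen.
; On BeginPlay it looks up its row name in DTInformationPieces, caches the title and text, and pre-creates an InfoPiece widget, printing a warning if the row is missing.
; ShowInfo and HideInfo toggle the widget in the viewport and track visibility.
; The title getter falls back to the row name for debugging.
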(event EventBeginPlay
  (bind _m_datatabletitle (Variables|Default|Getm_datatableTitle))
  ;[1 1 1] Read data
  (bind _returnvalue (Utilities|GetDataTableRow "/Game/Blueprints/Information/DTInformationPieces.DTInformationPieces" _m_datatabletitle)
    (:then
      (Variables|Default|Setm_informationDisplayTitle (.displaytitle _returnvalue))
      (Variables|Default|Setm_informationText (.content _returnvalue))
      ;[1 1 1] Create widget
      (bind _returnvalue_2 (UserInterface|CreateWidget "/Game/Blueprints/UI/InfoPiece.InfoPiece_C" (Game|GetPlayerController 0) (.displaytitle _returnvalue) (.content _returnvalue)))
      (Variables|Default|Setm_infoWidget _returnvalue_2))
    (:RowNotFound
      ;[1 1 1] Debugging warning
      (Development|PrintString (Utilities|String|Append "Could not find row: " (Utilities|String|ToString(Name) _m_datatabletitle)) true true "(R=0.000000,G=0.660000,B=1.000000,A=1.000000)" 5.0))))

(fn ShowInfo
  (bind _m_infowidget (Variables|Default|Getm_infoWidget)
    (:then
      (UserInterface|Viewport|AddtoViewport _m_infowidget 0)
      (Variables|Default|Setm_isInformationShowing true))
    (:else)))

(fn HideInfo
  (bind _m_infowidget (Variables|Default|Getm_infoWidget)
    (:then
      (Widget|RemovefromParent _m_infowidget)
      (Variables|Default|Setm_isInformationShowing false))
    (:else)))

(fn GetInformationTitle
  (bind _m_informationdisplaytitle (Variables|Default|Getm_informationDisplayTitle))
  ;[1 1 1] Get display name
  (if (Utilities|Array|IsEmpty _m_informationdisplaytitle)
    ;[1 1 1] If not display name found, return datatable title for debugging
    (return (Utilities|String|ToString(Name) (Variables|Default|Getm_datatableTitle)))
    (else
      (return _m_informationdisplaytitle))))

(fn GetIsInformationShowing
  (return (Variables|Default|Getm_isInformationShowing)))