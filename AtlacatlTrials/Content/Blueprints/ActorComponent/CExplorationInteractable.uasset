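; Actor component that makes its owner an interactable for an exploration goal.
; When interacted with while usable, it reports the target goal to FirstPersonGameMode, plays a sound at the owner and optionally disables the owner.
; An optional game mode binding makes it ignore a custom trace channel on the owner when that goal finishes, covering multiple objects that share one goal.
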(event Custom|ExplorationGoalFinished
  (params (aExplorationGoalCompleted :type EExplorationGoals%20Enum :default "NewEnumerator1"))
  ;[1 1 1] Disable object collision if exploration goal has already been completed, useful if multiple objects with same target goall
  (if (Utilities|Enum|Equal(Enum) aExplorationGoalCompleted (Variables|Default|Getm_targetGoal))
    (CallFunction|SetCollisionResponseAllComponents (Components|GetOwner) "ECC_GameTraceChannel2" "ECR_Ignore")))

(event EventInteract
  (params (aUser :type Actor%20Object%20Reference))
  (bind _returnvalue (Components|GetOwner))
  (bind _returnvalue_2 (Components|GetOwner))
  ;[1 1 1] Inform game mode that goal was finished
  (if (Variables|Default|Getm_canBeUsed)
    (bind _asfirst_person_game_mode (Utilities|Casting|CastToFirstPersonGameMode (Game|GetGameMode)))
    (Default|FinishedExplorationGoal _asfirst_person_game_mode (Variables|Default|Getm_targetGoal))
    (Utilities|IsValid _returnvalue_2
      (:Is%20Valid
        (Audio|PlaySoundatLocation (Variables|Default|Getm_soundToPlay) (Transformation|GetActorLocation _returnvalue_2) "0, 0, 0" 1.0 1.0 0.0 "/Game/AudioSettings/DefaultAttenuation.DefaultAttenuation" 0 0))
      (:Is%20Not%20Valid
        _))
    ;[1 1 1] Hide owner after use
    (if (Variables|Default|Getm_willHideOwnerOnUse)
      (Utilities|IsValid _returnvalue
        (:Is%20Valid
          (CallFunction|SetActorEnabled _returnvalue false))))))

(event EventBeginPlay
  ;[1 1 1] Disable object collision if exploration goal has already been completed, useful if multiple objects with same target goall
  (if (Variables|Default|Getm_willDisableCollisionOnSameGoalDone)
    (bind _asfirst_person_game_mode (Utilities|Casting|CastToFirstPersonGameMode (Game|GetGameMode)))
    (EventDispatchers|BindEventtoExplorationGoalFinished _asfirst_person_game_mode (delegate Custom|ExplorationGoalFinished))))